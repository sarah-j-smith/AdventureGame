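; BP_BasicFunctionalTest is a functional test that checks the adventure character moves in response to a point-and-click location click.
; Setup hands the character to the CommandManager and caches a marker's position, then start destroys the marker and sets up the camera.
; The first tick simulates a click through the CommandManager.
; Later ticks pass the test once the character nears the target, otherwise intermittently printing the distance for debugging.
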(event EventPrepareTest
  (Variables|/Script/AdventureGame.CommandManager|SetPlayerCharacter (Variables|Default|GetCommandManager) (Variables|Default|GetAdventureCharacter))
  (Variables|Default|SetWalkToLocation (Transformation|GetActorLocation (Variables|Default|GetLocationMarker))))

(event EventStartTest
  (Actor|DestroyActor (Variables|Default|GetLocationMarker))
  (Class|AdventureCharacter|SetupCamera (Variables|Default|GetAdventureCharacter)))

(event EventTick
  (params (DeltaSeconds :type Float%20%28single-precision%29))
  (bind _walktolocation (Variables|Default|GetWalkToLocation))
  (bind _adventurecharacter (Variables|Default|GetAdventureCharacter))
  (bind _capsulecomponent (Variables|/Script/Engine.Character|GetCapsuleComponent _adventurecharacter))
  (bind _returnvalue (Transformation|GetWorldLocation _capsulecomponent))
  (bind _returnvalue_2 (Math|Vector|Distance(Vector) _walktolocation _returnvalue))
  (if (Variables|Default|GetLocationClicked)
    (if (Class|AdvBlueprintFunctionLibrary|IsCharacterClosetoLocation (Variables|Default|GetWalkToLocation) (Variables|Default|GetAdventureCharacter) 5.0)
      (Class|FunctionalTest|FinishTest "Succeeded" "Player character moved in response to click")
      (else
        ;[0.15 0.15 0.15 0.5] Enable this to see distance on screen for debug
        (if (== (Math|Integer|%(Integer) (Math|Float|Truncate _returnvalue_2) 5) 0)
          (Development|PrintString (Utilities|String|ToString(Float) _returnvalue_2) true true "(R=0.000000,G=0.660000,B=1.000000,A=1.000000)" 2.0 "Distance to target"))))
    (else
      (Class|CommandManager|HandleLocationClicked (Variables|Default|GetCommandManager) (Variables|Default|GetWalkToLocation))
      (Variables|Default|SetLocationClicked true))))

(fn ConstructionScript)