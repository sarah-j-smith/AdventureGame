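; Functional test for the tower exterior of the point-and-click adventure, driving the player through looking at and pulling a poster to obtain the gherkin.
; A Tick-driven stage machine sends verb and hotspot clicks through CommandManager.
; Bound hotspot and inventory dispatchers set flags that advance stages, with the look step also checking the character's distance.
; The knife stage is a placeholder that immediately finishes the test as succeeded.
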(event Custom|PlayerInventoryChanged
  (params (ItemKind :type EItemKind%20Enum :default "None") (ItemDisposition :type EItemDisposition%20Enum :default "Unknown"))
  (Development|PrintString (Utilities|String|ToString(Text) (Utilities|Text|FormatText "\"Player inventory change {Operation} - {Item}" (Utilities|String|EnumtoString ItemDisposition) (Utilities|String|EnumtoString ItemKind))))
  (if (and (Utilities|Enum|Equal(Enum) ItemKind "Pickle") (Utilities|Enum|Equal(Enum) ItemDisposition "Added"))
    (Variables|Control|SetGherkinWasAdded true)))

(event Custom|OnReadyToCollectGherkin
  ;[0.15 0.15 0.15 0.5] Bind Events
  (Variables|Control|SetPosterHasBeenPulled true))

(event Custom|OnReadyToCollectKnife)

(event Custom|OnPosterLookSucceeded
  ;[0.15 0.15 0.15 0.5] Bind Events
  (Variables|Control|SetPosterHasBeenSeen true))

(event EventPrepareTest
  (bind _posterhotspot (Variables|Actors|GetPosterHotSpot))
  ;[0.15 0.15 0.15 0.5] Bind Events
  (EventDispatchers|BindEventtoOnPullDispatcher _posterhotspot (delegate Custom|OnReadyToCollectGherkin))
  (EventDispatchers|BindEventtoOnLookDispatcher _posterhotspot (delegate Custom|OnPosterLookSucceeded))
  (EventDispatchers|BindEventtoPlayerInventoryChanged (Class|AdvBlueprintFunctionLibrary|GetAdventureInstance) (EventDispatchers|CreateEvent :!event Custom|PlayerInventoryChanged)))

(event EventStartTest
  (Class|AdventureCharacter|SetupCamera (Variables|Actors|GetAdventureCharacter)))

(event EventTick
  (params (DeltaSeconds :type Float%20%28single-precision%29))
  (switch Utilities|FlowControl|Switch|SwitchonE_LevelStage (Variables|Control|GetTestStage)
    (:NewEnumerator0
      (if (Variables|Control|GetLookingAtPoster)
        (Utilities|CheckPosterSeen
          (:Success
            (Variables|Control|SetTestStage "NewEnumerator1")))
        (else
          (Utilities|GoLookPoster
            (:Out
              (Variables|Control|SetLookingAtPoster true))))))
    (:NewEnumerator1
      (if (Variables|Control|GetGettingGherkin)
        (if (Variables|Control|GetGherkinWasAdded)
          (Variables|Control|SetTestStage "NewEnumerator2"))
        (else
          (Utilities|GoPullPoster
            (:Out
              (Variables|Control|SetGettingGherkin true))))))
    (:NewEnumerator2
      (Class|FunctionalTest|FinishTest "Succeeded"))
    (:NewEnumerator8
      (Utilities|FlowControl|Delay 0.2)
      (Variables|Control|SetTestStage "NewEnumerator0"))))

(fn ConstructionScript)