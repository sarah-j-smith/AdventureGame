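; Point-and-click door hotspot between the tower exterior and interior, with a stone slab sprite that slides open.
; A timeline, rate-scaled to DoorOpenTime, drives the open ratio that offsets the sprite along Y and reverses to close.
; When the timeline finishes, the ratio sets the door state, and a nearly fully open slab is hidden.
; BeginPlay places an already-opened door in its open position.
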(event EventBeginPlay
  ;[0.15 0.15 0.15 0.5] Check the door state and if its open move the door sprite to the open position
  (Utilities|SetPlayRateforOpenTime
    (:Out
      (if (Utilities|Enum|Equal(Enum) (Variables|Default|GetDoorState) "Opened")
        (bind _output_get (Variables|Default|SetDoorOpenRatio 1.0))
        (Utilities|TowerDoorSetOpening _output_get)
        (else
          (Variables|Default|SetDoorOpenRatio 0.0))))))

(event EventOnOpen
  (|CallParentFunction) ; If the door can be opened, it will open
  (if (Utilities|Enum|Equal(Enum) (Variables|Default|GetDoorState) "Opened")
    (bind _dooropentrack (Timeline|Door_Open_Timeline Play)
      (:Update
        (Utilities|TowerDoorSetOpening _dooropentrack))
      (:Finished
        (Utilities|SetDoorStateTags
          (:Out
            ;[0.15 0.15 0.15 0.5] If the door is > 95% open hide the door slab sprite
            (if (> (Variables|Default|GetDoorOpenRatio) 0.95)
              (Class|PickUp|HideSprite))
            (Class|AdvBlueprintFunctionLibrary|ClearVerb))))
      (:PlaySound
        (Audio|PlaySound2D "/Game/PointAndClick/Sounds/FX/SoundWave_StoneDoor.SoundWave_StoneDoor" 1.0 1.0 0.0 0 0)))))

(event EventOnClose
  (bind _dooropentrack (Timeline|Door_Open_Timeline Reverse)
    (:Update
      (Utilities|TowerDoorSetOpening _dooropentrack))
    (:Finished
      (Utilities|SetDoorStateTags
        (:Out
          ;[0.15 0.15 0.15 0.5] If the door is > 95% open hide the door slab sprite
          (if (> (Variables|Default|GetDoorOpenRatio) 0.95)
            (Class|PickUp|HideSprite))
          (Class|AdvBlueprintFunctionLibrary|ClearVerb))))
    (:PlaySound
      (Audio|PlaySound2D "/Game/PointAndClick/Sounds/FX/SoundWave_StoneDoor.SoundWave_StoneDoor" 1.0 1.0 0.0 0 0))))

(fn ConstructionScript)